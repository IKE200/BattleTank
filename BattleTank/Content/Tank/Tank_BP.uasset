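; Tank Blueprint that lets the player aim the turret and barrel together with the camera through axis input.
; AimElevation pitches the SpringArm and barrel mesh, while AimAzimuth yaws the AzimuthGimbal and Turret.
; Both apply matching local rotations scaled by delta time at a fixed rate, with no angle clamping.
; BeginPlay, overlap, Tick and the construction script do nothing.
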(event EventBeginPlay)

(event Collision|EventActorBeginOverlap
  (params (OtherActor :type Actor%20Object%20Reference)))

(event EventTick
  (params (DeltaSeconds :type Float%20%28single-precision%29)))

(event Input|AxisEvents|InputAxisAimAzimuth
  (params (AxisValue :type Float%20%28single-precision%29))
  (bind _returnvalue (Utilities|Time|GetWorldDeltaSeconds))
  (bind _returnvalue_2 (* AxisValue _returnvalue 1e+02))
  ;[1 1 1] Move Camera Input
  (Transformation|AddLocalRotation (Variables|Default|GetAzimuth%20Gimbal) (Math|Rotator|MakeRotator 0.0 0.0 _returnvalue_2) false false)
  (Transformation|AddLocalRotation (Variables|Default|GetTurret) (Math|Rotator|MakeRotator 0.0 0.0 _returnvalue_2) false false))

(event Input|AxisEvents|InputAxisAimElevation
  (params (AxisValue :type Float%20%28single-precision%29))
  (bind _returnvalue (Utilities|Time|GetWorldDeltaSeconds))
  (bind _returnvalue_2 (* _returnvalue AxisValue 1e+02))
  ;[1 1 1] Move Camera Input
  (Transformation|AddLocalRotation (Variables|Default|GetSpringArm) (Math|Rotator|MakeRotator 0.0 _returnvalue_2 0.0) false false)
  (Transformation|AddLocalRotation (Variables|Default|Gettank_fbx_Barrel) (Math|Rotator|MakeRotator 0.0 _returnvalue_2 0.0) false false))

(fn ConstructionScript)